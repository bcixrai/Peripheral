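; BP_Animal is an animal actor with head and butt interaction components and an MBallHolder component.
; On BeginPlay it stores the first player's controlled pawn as its player, printing a debug message for success or failure.
; Each Tick it moves both interaction components to their mesh sockets and snaps MBallHolder to the Scene component's location, as the right-vector offset is zero.
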(event EventBeginPlay
  (bind _returnvalue (Game|GetPlayerController 0))
  (bind _returnvalue_2 (Pawn|GetControlledPawn _returnvalue))
  (Utilities|IsValid _returnvalue_2
    (:Is%20Valid
      (Class|Animal|SetPlayer _returnvalue_2)
      (Development|PrintString "Animal : Set Player" true true "(R=0.064219,G=1.000000,B=0.000000,A=1.000000)" 5.0))
    (:Is%20Not%20Valid
      (Development|PrintString "Animal : Found No Player" true true "(R=1.000000,G=0.008842,B=0.000000,A=1.000000)" 5.0))))

(event Collision|EventActorBeginOverlap
  (params (OtherActor :type Actor%20Object%20Reference)))

(event EventTick
  (params (DeltaSeconds :type Float%20%28single-precision%29))
  (bind _scene (Variables|Default|GetScene))
  (Utilities|FlowControl|Sequence
    (:then_1
      ;[1 1 1] Align With Bones
      (Utilities|FlowControl|Sequence
        (:then_0
          (Transformation|SetWorldLocation (Variables|Default|GetHeadInteraction) (Transformation|GetSocketLocation (Variables|Character|GetMesh) "HeadSocket") false false))
        (:then_1
          (Transformation|SetWorldLocation (Variables|Default|GetButtInteraction) (Transformation|GetSocketLocation (Variables|Character|GetMesh) "ButtSocket") false false))
        (:then_2
          (Transformation|SetWorldLocation (Variables|Default|GetmBallHolder) (+ (Transformation|GetWorldLocation _scene) (* (Math|Vector|GetRightVector _scene) "")) false false))))))

(fn ConstructionScript)