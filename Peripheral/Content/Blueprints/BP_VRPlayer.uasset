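; Player pawn for a painting game that runs in VR or normal mode, chosen by the game instance's peripheral setting, which configures camera, hands and floor placement.
; While painting, a ray from an origin picked by BCI mode moves a Niagara system across hit surfaces.
; Paint input toggles particle spawning or an erase volume on BP_Canvas, and ray-hit color boxes set color or eraser.
; A camera trace shows interact prompts.
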(event Custom|CheckForInteractables
  (bind _mcamera (Variables|Default|GetmCamera))
  ;[1 1 1] Check for Interactables
  (Variables|Default|SetShowInteractPrompt false)
  (Utilities|FlowControl|Sequence
    (:then_0
      (bind _outhit (Collision|LineTraceByChannel (Transformation|GetWorldLocation _mcamera) (+ (Transformation|GetWorldLocation _mcamera) (* (Math|Vector|GetForwardVector _mcamera) 1.5e+02)) "TraceTypeQuery1" false 0 "None"))
      (Utilities|IsValid (.HitActor (Collision|BreakHitResult _outhit))
        (:Is%20Valid
          (Utilities|Casting|CastToInteractable (.HitActor (Collision|BreakHitResult _outhit))
            (:then
              (Development|PrintString "Hello")
              (Variables|Default|SetShowInteractPrompt true))
            (:CastFailed
              (Variables|Default|SetShowInteractPrompt (> (Utilities|Array|Length (Class|Actor|GetComponentsbyInterface (.HitActor (Collision|BreakHitResult _outhit)) "/Script/Peripheral.Interactable")) 0)))))))
    (:then_2
      (if (Variables|Default|GetShowInteractPrompt)
        (Widget|SetVisibility (Variables|Default|GetInteractPrompt) "Visible")
        (else
          (Widget|SetVisibility (Variables|Default|GetInteractPrompt) "Hidden"))))))

(event Custom|Painting
  (bind _map_vr_paint_origin (Variables|Default|GetMap_VR_Paint_Origin))
  (bind _bcimode (Variables|Default|GetBCIMode))
  (bind _map_normal_paint_origin (Variables|Default|GetMap_NORMAL_Paint_Origin))
  (bind _bcimode_2 (Variables|Default|GetBCIMode))
  (bind _niagara_system (Variables|Default|GetNiagara%20System))
  (bind (_value _returnvalue) (Utilities|Map|Find _map_normal_paint_origin _bcimode_2))
  (bind (_value_2 _returnvalue_2) (Utilities|Map|Find _map_vr_paint_origin _bcimode))
  (bind _returnvalue_3 (Transformation|GetWorldLocation _value_2))
  (bind _returnvalue_4 (Transformation|GetWorldLocation _value_2))
  (bind _returnvalue_5 (Transformation|GetWorldLocation _value))
  (if (Variables|Default|GetCurrent%20Painting)
    (bind _returnvalue_6 (Class|PeripheralGameInstance|GetPeripheralModefromInstance (Variables|Default|GetGI_Peripheral)))
    (if (Utilities|Enum|Equal(Enum) _returnvalue_6 "VR")
      ;[1 1 1] Painting in VR
      (if _returnvalue_2
        (switch Utilities|FlowControl|Switch|SwitchonEBCIMode (Variables|Default|GetBCIMode)
          (:NO_BCI
            (bind (_outhit_location _outhit_normal _outhit_hitactor) (|SHHOTRAYCASTVRNOBCI _returnvalue_3 (+ _returnvalue_3 (* (* (Math|Vector|GetRightVector (Transformation|GetWorldRotation _value_2)) -1.0) 4e+03)) (Variables|Default|GetObjectTypes)))
            (Variables|Default|SetOut%20Hit%20Location _outhit_location)
            (Variables|Default|SetOut%20Hit%20Normal _outhit_normal)
            (Variables|Default|SetOut%20Hit%20Hit%20Actor _outhit_hitactor))
          (:BCI
            (bind (_out_hit_location _out_hit_normal _out_hit_hit_actor) (|SHOTRAYCASTVRBCI _returnvalue_4 (+ _returnvalue_4 (* (Math|Vector|GetForwardVector _value_2) 4e+03)) (Variables|Default|GetObjectTypes)))
            (Variables|Default|SetOut%20Hit%20Location _out_hit_location)
            (Variables|Default|SetOut%20Hit%20Normal _out_hit_normal)
            (Variables|Default|SetOut%20Hit%20Hit%20Actor _out_hit_hit_actor)))
        (bind _asbp_color_box (Utilities|Casting|CastToBP_ColorBox (Variables|Default|GetOut%20Hit%20Hit%20Actor))
          (:then
            (CallFunction|SetBrushColor _asbp_color_box)
            (Variables|Default|SetLooking%20at%20Canvas false))
          (:CastFailed
            (Transformation|SetWorldLocation (Variables|Default|GetNiagara%20System) (Math|Vector|MakeVector (- (.x (Variables|Default|GetOut%20Hit%20Location)) 1.0) (.y (Variables|Default|GetOut%20Hit%20Location)) (.z (Variables|Default|GetOut%20Hit%20Location))) false false)
            (Niagara|SetNiagaraVariable(Vector3) (Variables|Default|GetNiagara%20System) "Facing" (Variables|Default|GetOut%20Hit%20Normal))
            (if (Utilities|Enum|Equal(Enum) (Utilities|GetDisplayName (Variables|Default|GetOut%20Hit%20Hit%20Actor)) "BP_Canvas")
              (Variables|Default|SetLooking%20at%20Canvas true)
              (else
                (Variables|Default|SetLooking%20at%20Canvas false)))))
        (else
          (Development|PrintString "PlayerBP : NO VR PAINT ORIGIN FOUND" true true "(R=1.000000,G=0.012564,B=0.000000,A=1.000000)" 5.0)))
      (else
        ;[1 1 1] Painting Raytracing without VR
        (if _returnvalue
          (bind _outhit (Collision|LineTraceForObjects _returnvalue_5 (+ _returnvalue_5 (* (Math|Vector|GetForwardVector _value) 1e+04)) (Variables|Default|GetObjectTypes) false 0 "ForDuration" true "(R=1.000000,G=0.000000,B=0.000000,A=1.000000)" "(R=0.000000,G=1.000000,B=0.000000,A=1.000000)" 0.0))
          (Variables|Default|SetOut%20Hit%20Location (.location _outhit))
          (Transformation|SetWorldLocation _niagara_system (Math|Vector|MakeVector (- (.x (Variables|Default|GetOut%20Hit%20Location)) 1.0) (.y (Variables|Default|GetOut%20Hit%20Location)) (.z (Variables|Default|GetOut%20Hit%20Location))) false false)
          (Niagara|SetNiagaraVariable(Vector3) _niagara_system "Facing" (.normal _outhit))
          (bind _asbp_color_box_2 (Utilities|Casting|CastToBP_ColorBox (.hitactor _outhit))
            (:then
              (CallFunction|SetBrushColor _asbp_color_box_2)
              (Variables|Default|SetLooking%20at%20Canvas false :!label _label))
            (:CastFailed
              (if (Utilities|Enum|Equal(Enum) (Utilities|GetDisplayName (.hitactor _outhit)) "BP_Canvas")
                (Variables|Default|SetLooking%20at%20Canvas true)
                (else
                  (goto _label)))))
          (else
            (Development|PrintString "PlayerBP : NO NORMAL PAINT ORIGIN FOUND" true true "(R=1.000000,G=0.012564,B=0.000000,A=1.000000)" 5.0)))))))

(event Custom|Set%20BCI%20Mode
  ;[1 1 1] Update BCI mode for Blueprint Every frame
  (bind _returnvalue (Class|VRPlayer|GetBCIModefromPlayer))
  (Variables|Default|SetBCIMode _returnvalue))

(event Custom|Set%20Brush%20Color
  (params (ColorBox :type BP%20Color%20Box%20Object%20Reference))
  ;[1 1 1] Set Brush COlor
  (if (Variables|/Game/Niagara/BP_ColorBox.BP_ColorBox_C|GetEraser ColorBox)
    (Variables|Default|SetEraser true)
    (else
      (Class|NiagaraComponent|SetVariableInt (Variables|Default|GetNiagara%20System) "User.ColorSelector" (Variables|/Game/Niagara/BP_ColorBox.BP_ColorBox_C|GetNiagraIndex ColorBox))
      (Variables|Default|SetEraser false))))

(event EventBeginPlay
  (bind _returnvalue (Transformation|GetActorLocation))
  (bind _map_vr_paint_origin (Variables|Default|GetMap_VR_Paint_Origin))
  (bind _map_normal_paint_origin (Variables|Default|GetMap_NORMAL_Paint_Origin))
  (bind _mcamera (Variables|Default|GetmCamera))
  (bind _mcamera_2 (Variables|Default|GetmCamera))
  (Utilities|FlowControl|Sequence
    (:then_0
      ;[1 1 1] Get Peripheral Mode
      (bind _asgi_peripheral (Utilities|Casting|CastToGI_Peripheral (Game|GetGameInstance)))
      (bind _output_get (Variables|Default|SetGI_Peripheral _asgi_peripheral))
      (bind _returnvalue_2 (Class|PeripheralGameInstance|GetPeripheralModefromInstance _output_get))
      (Variables|Default|SetMode _returnvalue_2))
    (:then_1
      ;[1 1 1] HUD
      (bind _returnvalue_3 (UserInterface|CreateWidget "/Game/Blueprints/UW_PlayerHUD.UW_PlayerHUD_C"))
      (bind _output_get_2 (Variables|Default|SetHUD _returnvalue_3))
      (UserInterface|Viewport|AddtoViewport _output_get_2 0))
    (:then_2
      ;[1 1 1] Interaction Prompt
      (bind _returnvalue_4 (UserInterface|CreateWidget "/Game/Blueprints/UW_InteractPrompt.UW_InteractPrompt_C"))
      (bind _output_get_3 (Variables|Default|SetInteractPrompt _returnvalue_4))
      (UserInterface|Viewport|AddtoViewport _output_get_3 0))
    (:then_3
      ;[1 1 1] Hide Hands Mesh Based on mdoe
      (bind _returnvalue_5 (Class|PeripheralGameInstance|GetPeripheralModefromInstance (Variables|Default|GetGI_Peripheral)))
      (switch Utilities|FlowControl|Switch|SwitchonEPeripheralMode _returnvalue_5
        (:NORMAL
          (Variables|/Script/HeadMountedDisplay.MotionControllerComponent|SetbDisplayDeviceModel (Variables|Default|GetmLeftMC) false)
          (Variables|/Script/HeadMountedDisplay.MotionControllerComponent|SetbDisplayDeviceModel (Variables|Default|GetmRightMC) false))
        (:VR
          (Variables|/Script/HeadMountedDisplay.MotionControllerComponent|SetbDisplayDeviceModel (Variables|Default|GetmLeftMC) true)
          (Variables|/Script/HeadMountedDisplay.MotionControllerComponent|SetbDisplayDeviceModel (Variables|Default|GetmRightMC) true))))
    (:then_4
      ;[1 1 1] VR tracking
      (if (Class|HeadMountedDisplayFunctionLibrary|IsHeadMountedDisplayEnabled)
        (Class|HeadMountedDisplayFunctionLibrary|SetTrackingOrigin "Floor")
        (Development|ExecuteConsoleCommand "vr.PixelDensity 1" 0)
        (Input|EnableInput (Game|GetPlayerController 0))))
    (:then_5
      ;[1 1 1] Change location based On Normal or VR mode
      (Utilities|FlowControl|Sequence
        (:then_0
          (bind _returnvalue_6 (Class|PeripheralGameInstance|GetPeripheralModefromInstance (Variables|Default|GetGI_Peripheral)))
          (switch Utilities|FlowControl|Switch|SwitchonEPeripheralMode _returnvalue_6
            (:NORMAL
              (Development|PrintString "IN NORMAL MODE" true true "(R=0.011214,G=1.000000,B=0.000000,A=1.000000)" 5.0))
            (:VR
              (Development|PrintString "IN VR MODE" true true "(R=0.018355,G=1.000000,B=0.000000,A=1.000000)" 5.0)
              (bind (_outhit _returnvalue_7) (Collision|LineTraceByChannel _returnvalue (+ _returnvalue (* (* (Transformation|GetActorUpVector) -1.0) 10000)) "TraceTypeQuery1" false 0 "None"))
              (if _returnvalue_7
                (Transformation|SetActorLocation (.Location (Collision|BreakHitResult _outhit)) false false)
                (else
                  (Development|PrintString "Found No Floor To Attach To" true true "(R=1.000000,G=0.000000,B=0.007180,A=1.000000)" 5.0))))))
        (:then_1
          (Development|PrintString "Moved Player Based on Mode" true true "(R=0.030624,G=1.000000,B=0.000000,A=1.000000)" 5.0))))
    (:then_6
      ;[1 1 1] Set Camera pawn control rotation and hmd
      (bind _asperipheral_game_instance (Utilities|Casting|CastToPeripheralGameInstance (Game|GetGameInstance)))
      (bind _returnvalue_8 (Class|PeripheralGameInstance|GetPeripheralModefromInstance _asperipheral_game_instance))
      (if (Utilities|Enum|Equal(Enum) _returnvalue_8 "VR")
        (Variables|/Script/Engine.CameraComponent|SetbUsePawnControlRotation _mcamera false)
        (Variables|/Script/Engine.CameraComponent|SetbLockToHmd _mcamera true)
        (else
          (Variables|/Script/Engine.CameraComponent|SetbUsePawnControlRotation _mcamera_2 true)
          (Variables|/Script/Engine.CameraComponent|SetbLockToHmd _mcamera_2 false))))
    (:then_7
      (bind _returnvalue_9 (Niagara|SpawnSystematLocation "/Game/Niagara/Painting_NS.Painting_NS" (Variables|Default|GetOut%20Hit%20Location)))
      (Variables|Default|SetNiagara%20System _returnvalue_9))
    (:then_8
      (bind _asperipheral_game_instance_2 (Utilities|Casting|CastToPeripheralGameInstance (Game|GetGameInstance)))
      (bind _returnvalue_10 (Class|PeripheralGameInstance|GetPeripheralModefromInstance _asperipheral_game_instance_2))
      (Variables|Default|SetVRenabled (Utilities|Enum|Equal(Enum) _returnvalue_10 "VR"))
      (Variables|Default|SetNormalEnabled (Utilities|Enum|Equal(Enum) _returnvalue_10 "NORMAL")))
    (:then_9
      ;[1 1 1] Set PAINTING ORIGINS
      (Utilities|Map|Add _map_vr_paint_origin "NO_BCI" (Variables|Default|GetmRightMC))
      (Utilities|Map|Add _map_vr_paint_origin "BCI" (Variables|Default|GetmBCIHand)))
    (:then_10
      ;[1 1 1] NORMAL PAINTING ORIGIN
      (Utilities|Map|Add _map_normal_paint_origin "NO_BCI" (Variables|Default|GetmCamera))
      (Utilities|Map|Add _map_normal_paint_origin "BCI" (Variables|Default|GetmBCIHand)))))

(event Collision|EventActorBeginOverlap
  (params (OtherActor :type Actor%20Object%20Reference)))

(event EventTick
  (params (DeltaSeconds :type Float%20%28single-precision%29))
  (Utilities|FlowControl|Sequence
    (:then_0
      (CallFunction|SetBCIMode))
    (:then_1
      (CallFunction|CheckforInteractables))
    (:then_2
      (CallFunction|Painting))))

(event Input|ActionEvents|InputActionPaint
  (params (Key :type Key%20Structure :default "None"))
  (bind _out_hit_location (Variables|Default|GetOut%20Hit%20Location))
  ;[1 1 1] DRaw and Erase
  (:Pressed
    (Variables|Default|SetCurrent%20Painting true)
    (if (Variables|Default|GetLooking%20at%20Canvas)
      (if (Variables|Default|Geteraser)
        (Class|NiagaraComponent|SetVariableBool (Variables|Default|GetNiagara%20System) "User.KillVolume" true)
        (else
          (Class|NiagaraComponent|SetVariableBool (Variables|Default|GetNiagara%20System) "User.KillVolume" false)
          (if (Utilities|IsValid (Variables|Default|GetNiagara%20System))
            (Transformation|SetWorldLocation (Variables|Default|GetNiagara%20System) _out_hit_location false false)
            (Utilities|FlowControl|Delay 0.05)
            (Niagara|SetNiagaraVariable(Float) (Variables|Default|GetNiagara%20System) "User.spawnrate" 4e+02)
            (else
              (bind _returnvalue (Niagara|SpawnSystematLocation "/Game/Niagara/Painting_NS.Painting_NS" _out_hit_location))
              (Variables|Default|SetNiagara%20System _returnvalue)))))))
  (:Released
    (Variables|Default|SetCurrent%20Painting false)
    (Niagara|SetNiagaraVariable(Float) (Variables|Default|GetNiagara%20System) "User.spawnrate" 0.0)
    (Class|NiagaraComponent|SetVariableBool (Variables|Default|GetNiagara%20System) "User.KillVolume" false)))

(event Input|KeyboardEvents|E
  (params (Key :type Key%20Structure :default "None"))
  (:Pressed
    (if (Variables|Default|Geteraser)
      (Variables|Default|Seteraser false)
      (else
        (Variables|Default|Seteraser true)))))

(fn ConstructionScript)

(fn GetGrabComponentsNearMotionController
  (params (MotionController :type Motion%20Controller%20Component%20Object%20Reference))
  (Development|PrintString "Grab Near Motion")
  (Utilities|FlowControl|Sequence
    (:then_0
      ;[1 1 1] Get Grab Position and Sphere trace
      (bind _output_get (LocalVariables|SetLocalGripPosition (Transformation|GetWorldLocation MotionController)))
      (bind (_outhit _returnvalue) (Collision|SphereTraceForObjects _output_get _output_get (Variables|Default|GetGrabRadiusFromGripPosition) (Utilities|Array|MakeArray "ObjectTypeQuery4") false 0 "None"))
      (if _returnvalue
        ;[1 1 1] Does the actors hit have a grab component
        (if (> (Utilities|Array|Length (Actor|GetComponentsByClass (.HitActor (Collision|BreakHitResult _outhit)) "/Script/Peripheral.GrabComponent")) 0)
          (bind _output_get_2 (LocalVariables|SetLocalComponents (Actor|GetComponentsByClass (.HitActor (Collision|BreakHitResult _outhit)) "/Script/Peripheral.GrabComponent")))
          (for _array_element _output_get_2
            (if (<= (Math|Vector|VectorLengthSquared (- (Transformation|GetWorldLocation _array_element) (LocalVariables|GetLocalGripPosition))) (LocalVariables|GetLocalNearestComponentDistance))
              (LocalVariables|SetLocalNearestComponentDistance (Math|Vector|VectorLengthSquared (- (Transformation|GetWorldLocation _array_element) (LocalVariables|GetLocalGripPosition))))
              (LocalVariables|SetLocalNearestGrabComponent _array_element))))
        (else
          (Development|PrintString "No Objects Sphere Traced" true true "(R=1.000000,G=0.050593,B=0.000000,A=1.000000)"))))
    (:then_1
      ;[1 1 1] If a nearby has been found this will be the nearest
      (return (LocalVariables|GetLocalNearestGrabComponent)))))