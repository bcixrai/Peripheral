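; VR player controller that places the player at the level's start and handles debug and menu keys.
; BeginPlay teleports the VRPlayer pawn to the first BP_PlayerStartLocationActor found.
; Escape or | pauses and F1 advances maps through GI_Peripheral.
; Unfinished stubs include the 1-key Animal/Ball loop, PausePlayer, and a local OSC "BCI Server" whose CreateServers event is uncalled here and whose bundle handler only prints.
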(event Custom|Create%20Servers
  (Utilities|FlowControl|Sequence
    (:then_0
      (bind _returnvalue (Class|OSCManager|CreateOSCServer "127.0.0.1" 1601 false false "BCI Server" 0))
      (Variables|Default|SetBCI%20Server _returnvalue))
    (:then_1
      (EventDispatchers|AssignOnOscBundleReceived (Variables|Default|GetBCI%20Server) (delegate Custom|BCI%20Bundle)))))

(event Custom|BCI%20Bundle
  (params (Bundle :type OSC%20Bundle%20Structure%20%28by%20ref%29) (IPAddress :type String) (Port :type Integer))
  (Development|PrintString "BCI BUNDLE" true true "(R=0.000000,G=0.660000,B=1.000000,A=1.000000)" 2.0 "BCIBUNDLE")
  (bind _returnvalue (Class|OSCManager|GetMessagesfromBundle Bundle))
  (for _array_element _returnvalue
    _))

(event EventBeginPlay
  (Utilities|FlowControl|Sequence
    (:then_0
      ;[1 1 1] Change player location
      (bind _outactors (Actor|GetAllActorsOfClass "/Game/Blueprints/BP_PlayerStartLocationActor.BP_PlayerStartLocationActor_C"))
      (if (> (Utilities|Array|Length _outactors) 0)
        (Development|PrintString (Utilities|String|Append "PC : Found " (Utilities|String|ToString(Integer) (Utilities|Array|Length _outactors)) " start locations, using 0th") true true "(R=0.000000,G=0.660000,B=1.000000,A=1.000000)" 5.0)
        (bind _asvrplayer (Utilities|Casting|CastToVRPlayer (Game|Player|GetPlayerPawn 0))
          (:then
            (Transformation|SetActorLocation _asvrplayer (Transformation|GetActorLocation (Utilities|Array|Get(acopy) _outactors)) false true)
            (Transformation|SetActorRotation _asvrplayer (Transformation|GetActorRotation (Utilities|Array|Get(acopy) _outactors))))
          (:CastFailed
            (Development|PrintString "PC : No Player" true true "(R=1.000000,G=0.027538,B=0.000000,A=1.000000)" 6.0)))))))

(event EventTick
  (params (DeltaSeconds :type Float%20%28single-precision%29)))

(event Input|KeyboardEvents||
  (params (Key :type Key%20Structure :default "None"))
  ;[1 1 1] Pausing
  (:Pressed
    (bind _asgi_peripheral (Utilities|Casting|CastToGI_Peripheral (Game|GetGameInstance)))
    (Default|Pause _asgi_peripheral)))

(event Input|KeyboardEvents|Escape
  (params (Key :type Key%20Structure :default "None"))
  ;[1 1 1] Pausing
  (:Pressed
    (bind _asgi_peripheral (Utilities|Casting|CastToGI_Peripheral (Game|GetGameInstance)))
    (Default|Pause _asgi_peripheral)))

(event Input|KeyboardEvents|F1
  (params (Key :type Key%20Structure :default "None"))
  (:Pressed
    (bind _asgi_peripheral (Utilities|Casting|CastToGI_Peripheral (Game|GetGameInstance)))
    (Default|NextMap _asgi_peripheral)))

(event Input|KeyboardEvents|1
  (params (Key :type Key%20Structure :default "None"))
  (:Pressed
    (bind _outactors (Actor|GetAllActorsOfClass "/Script/Peripheral.Animal"))
    (for _array_element _outactors
      (bind _outactors_2 (Actor|GetAllActorsOfClass "/Script/Peripheral.Ball"))
      (if (> (Utilities|Array|Length _outactors_2) 0)
        _))))

(fn ConstructionScript)

(fn PausePlayer
  (params (paused :type Boolean))
  (if paused
    _))