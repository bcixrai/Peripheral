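; Game instance that configures the build's peripheral and BCI modes and registers the game's profiles and levels at startup.
; Init hard-sets VR and BCI modes, toggles the HMD by console command, then adds placeholder profiles, the lobby, activity maps and always-on extra entries.
; Pause toggles the pause widget along with cursor and input mode.
; NextMap cycles through the registered level list, wrapping to the first.
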(event EventInit
  ;[1 1 1] THIS DECIDES THE MODE TOO BUILD FOR
  (Class|PeripheralGameInstance|SetPeripheralModefromInstance "VR")
  ;[1 1 1] Enable BCI Mode
  (Class|PeripheralGameInstance|SetBCIModefromInstance "BCI")
  (Utilities|FlowControl|Sequence
    (:then_0
      ;[1 1 1] Set Mode
      (bind _returnvalue (Class|PeripheralGameInstance|GetPeripheralModefromInstance))
      (if (Utilities|Enum|Equal(Enum) _returnvalue "VR")
        (Development|ExecuteConsoleCommand "hmd enable" 0)
        (else
          (Development|ExecuteConsoleCommand "hmd disable" 0))))
    (:then_1
      ;[1 1 1] Profiles
      (Class|PeripheralGameInstance|AddProfile (Utilities|Struct|MakeProfile "Adam" "Adam" "Very bald" "/Game/Assets_+_Textures/Assets/Library/Books_and_drinks/Var3/Redstem_Colocasia_4K_Albedo.Redstem_Colocasia_4K_Albedo"))
      (Class|PeripheralGameInstance|AddProfile (Utilities|Struct|MakeProfile "Santa" "Adam" "Sees you when you're sleeping" "/Game/Assets_+_Textures/Textures/SHELF_/shelf_metal_handle_OcclusionRoughnessMetallic.shelf_metal_handle_OcclusionRoughnessMetallic")))
    (:then_2
      ;[1 1 1] Lobby Map
      (Class|PeripheralGameInstance|AddLevel (Utilities|Struct|MakePeripheralLevel "Lobby" "Lobby" "M_Lobby" "/Game/Levels/MicrosoftTeams-image__4_.MicrosoftTeams-image__4_")))
    (:then_3
      ;[1 1 1] Level Maps
      (Class|PeripheralGameInstance|AddLevel (Utilities|Struct|MakePeripheralLevel "Wood Stacking" "Relaxing wood stacking" "M_WoodStacking" "/Game/Levels/MicrosoftTeams-image__2_.MicrosoftTeams-image__2_"))
      (Class|PeripheralGameInstance|AddLevel (Utilities|Struct|MakePeripheralLevel "Animal Petting" "Play with an animal" "M_AnimalPetting" "/Game/Levels/MicrosoftTeams-image__5_.MicrosoftTeams-image__5_"))
      (Class|PeripheralGameInstance|AddLevel (Utilities|Struct|MakePeripheralLevel "Music Box" "Music Level" " M_MusicBox" "/Game/Levels/MicrosoftTeams-image__6_.MicrosoftTeams-image__6_"))
      (Class|PeripheralGameInstance|AddLevel (Utilities|Struct|MakePeripheralLevel "Painting" "Paint in VR or with Brain" "M_Painting" "/Game/Levels/MicrosoftTeams-image__3_.MicrosoftTeams-image__3_")))
    (:then_4
      ;[1 1 1] Extras
      (if true
        (Class|PeripheralGameInstance|AddLevel (Utilities|Struct|MakePeripheralLevel "Main Menu" "The main menu" "M_MainMenu" "/Game/Assets_+_Textures/Textures/BOOK/books_texture3011.books_texture3011"))
        (Class|PeripheralGameInstance|AddLevel (Utilities|Struct|MakePeripheralLevel "Adam" "The level Adam has been testing on" "AdamMap" "/Game/Assets_+_Textures/Textures/LAMP/Lamp_lamp_base_OcclusionRoughnessMetallic.Lamp_lamp_base_OcclusionRoughnessMetallic"))))))

(fn Pause
  (Utilities|IsValid (Variables|Default|GetPauseScreen)
    (:Is%20Valid
      (Widget|RemovefromParent (Variables|Default|GetPauseScreen))
      (Variables|Default|SetPauseScreen 0)
      (Variables|/Script/Engine.PlayerController|SetbShowMouseCursor (Game|GetPlayerController 0) false)
      (Input|SetInputModeGameOnly (Game|GetPlayerController 0)))
    (:Is%20Not%20Valid
      (bind _returnvalue (UserInterface|CreateWidget "/Game/PauseScreen/UW_PauseScreen.UW_PauseScreen_C"))
      (bind _output_get (Variables|Default|SetPauseScreen _returnvalue))
      (UserInterface|Viewport|AddtoViewport _output_get 0)
      (Variables|/Script/Engine.PlayerController|SetbShowMouseCursor (Game|GetPlayerController 0) true)
      (Input|SetInputModeUIOnly (Game|GetPlayerController 0) (Variables|Default|GetPauseScreen) "DoNotLock"))))

(fn NextMap
  (Math|Integer|IncrementInt (Variables|Default|GetCurrentMap)
    (:%20%20
      (bind _returnvalue (Class|PeripheralGameInstance|GetAllLevelsArray))
      (if (>= (Variables|Default|GetCurrentMap) (Utilities|Array|Length _returnvalue))
        (Variables|Default|SetCurrentMap 0))
      (Game|OpenLevel(byName) (.mLevelName (Utilities|Struct|BreakPeripheralLevel (Utilities|Array|Get(acopy) _returnvalue (Variables|Default|GetCurrentMap))))))))